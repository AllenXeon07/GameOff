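; Main game mode that runs a timed, scored round, with the in-game HUD and looping background music.
; Tick restarts music by counting down its duration, queues the Rush track once time runs low, updates the score widget and triggers PC_Player's GameOver at zero.
; RandomEvent randomly adds time or temporarily speeds up or slows the player.
; Helper functions add score and check whether any BP_RandomBox exists.
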(event `self.ReceiveBeginPlay`
  (bind _nextsong (`self.NextSong`))
  (`GameplayStatics.PlaySound2D` _nextsong 1.0 1.0 0.0 null null)
  (set `self.Duration` (`SoundBase.Duration` _nextsong))
  (bind _returnvalue (`|CreateWidget` "/Game/Player/WB_InGame.WB_InGame_C"))
  (set `self.InGameWidget` _returnvalue)
  (`UserWidget.AddToViewport` _returnvalue 0)
  (bind _aspc_player (cast `/Game/Player/PC_Player` (`GameplayStatics.GetPlayerController` 0)))
  (set `self.PC` _aspc_player))

(event `self.ReceiveTick`
  (params (DeltaSeconds :type "Float (single-precision)"))
  (bind _nextsong (`self.NextSong`))
  (bind _returnvalue (`KismetMathLibrary.FMax` (- (`self.TimeRemain`) DeltaSeconds)))
  (`|ExecutionSequence`
    (:`then_0`
      (bind _output_get (set `self.Duration` (- (`self.Duration`) DeltaSeconds)))
      (if (<= _output_get 0.0)
        (`GameplayStatics.PlaySound2D` _nextsong 1.0 1.0 0.0 null null)
        (set `self.Duration` (`SoundBase.Duration` _nextsong))))
    (:`then_1`
      (if (and (< (`self.TimeRemain`) 180.0) (not (`self.Frenzy`)))
        (set `self.Frenzy` true)
        (set `self.NextSong` "/Game/Sound/rush.rush")))
    (:`then_2`
      (`/Game/Player/WB_InGame.SetScore` (`self.InGameWidget`) (`KismetMathLibrary.Conv_IntToDouble` (`self.Score`)))
      (if (`self.Play?`)
        (set `self.TimeRemain` _returnvalue)
        (if (== _returnvalue 0.0)
          (set `self.Play?` false)
          (`/Game/Player/PC_Player.GameOver` (`self.PC`) (`KismetMathLibrary.Conv_IntToDouble` (`self.Score`))))))))

(event `RandomEvent`
  (switch `int` (`KismetMathLibrary.RandomIntegerInRange` 0 2)
    (:`0`
      (set `self.TimeRemain` (+ (`self.TimeRemain`) 15.0)))
    (:`1`
      (`/Game/Player/PC_Player.SetSpeed` (`self.PC`) 750.0)
      (`KismetSystemLibrary.Delay` 6.0)
      (`/Game/Player/PC_Player.SetSpeed` (`self.PC`) 500.0))
    (:`2`
      (`/Game/Player/PC_Player.SetSpeed` (`self.PC`) 200.0)
      (`KismetSystemLibrary.Delay` 15.0)
      (`/Game/Player/PC_Player.SetSpeed` (`self.PC`) 500.0))))

(fn `AddScore`
  (params (Score :type "Float (double-precision)"))
  (set `self.Score` (+ (`self.Score`) Score)))

(fn `CheckRandom`
  (returns (Exist :type Boolean))
  (bind _outactors (`GameplayStatics.GetAllActorsOfClass` "/Game/Object/BP_RandomBox.BP_RandomBox_C"))
  (return (> (`KismetArrayLibrary.Array_Length` _outactors) 0)))

(fn `UserConstructionScript`)