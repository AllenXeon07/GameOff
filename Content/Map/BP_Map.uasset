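; BP_Map is a map generator actor that spawns a grid of BP_Floor tiles with BP_Wall pieces along three edges.
; GenerateMap measures tile size by spawning a temporary floor, doubling the distance to its Arrow component, then destroying it.
; Nested row and column loops place tiles from the actor's location, adding half-tile-offset walls on both Y edges and the +X edge, leaving -X open.
; BeginPlay and the construction script are empty.
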(event `self.ReceiveBeginPlay`)

(fn `GenerateMap`
  (bind _returnvalue (`self.K2_GetActorLocation`))
  (bind _size (`self.Size`))
  (bind _returnvalue_2 (/ (`self.Size`) 2.0))
  (bind _returnvalue_3 (`|SpawnActorFromClass` "/Game/Map/BP_Floor.BP_Floor_C" (`KismetMathLibrary.MakeTransform` _returnvalue) "Undefined" "MultiplyWithRoot" null null))
  (set `self.Size` (* (`KismetMathLibrary.VSize` (- _returnvalue (`SceneComponent.K2_GetComponentLocation` (`/Game/Map/BP_Floor.Arrow` _returnvalue_3)))) 2.0))
  (`self.K2_DestroyActor` _returnvalue_3)
  (for _index (range (+ (`self.RowLength`) 1))
    (for _index_2 (range (+ (`self.ColumnLength`) 1))
      (bind _returnvalue_4 (+ (`self.K2_GetActorLocation`) (`KismetMathLibrary.MakeVector` (* _index_2 _size) (* _index _size))))
      (`|SpawnActorFromClass` "/Game/Map/BP_Floor.BP_Floor_C" (`KismetMathLibrary.MakeTransform` _returnvalue_4) "Undefined" "MultiplyWithRoot" null null)
      (if (== _index 0)
        (bind _x (.x _returnvalue_4))
        (bind _y (.y _returnvalue_4))
        (bind _z (.z _returnvalue_4))
        (`|SpawnActorFromClass` "/Game/Map/BP_Wall.BP_Wall_C" (`KismetMathLibrary.MakeTransform` (`KismetMathLibrary.MakeVector` _x (- _y _returnvalue_2) _z)) "Undefined" "MultiplyWithRoot" null null))
      (if (== _index (`self.RowLength`))
        (`|SpawnActorFromClass` "/Game/Map/BP_Wall.BP_Wall_C" (`KismetMathLibrary.MakeTransform` (`KismetMathLibrary.MakeVector` _x (+ _y _returnvalue_2) _z) (struct :`Yaw` 180.0)) "Undefined" "MultiplyWithRoot" null null))
      (if (== _index_2 (`self.ColumnLength`))
        (`|SpawnActorFromClass` "/Game/Map/BP_Wall.BP_Wall_C" (`KismetMathLibrary.MakeTransform` (`KismetMathLibrary.MakeVector` (+ _x _returnvalue_2) _y _z) (struct :`Yaw` 90.0)) "Undefined" "MultiplyWithRoot" null null)))))

(fn `UserConstructionScript`)