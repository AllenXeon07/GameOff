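; Spawner actor that replaces its BP_Box a few seconds after the current one leaves its Box volume.
; End overlap of the spawned box clears the reference and sets Taken, which Tick polls to call SpawnBox after a Delay.
; SpawnBox creates a box at the volume's location with random Mass and Point values, clears Taken and disables physics simulation on its cube.
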(event `self.ReceiveTick`
  (params (DeltaSeconds :type "Float (single-precision)"))
  (if (`self.taken`)
    (`KismetSystemLibrary.Delay` 6.0)
    (`self.SpawnBox`)))

(event `SpawnBox`
  (bind _returnvalue (`|SpawnActorFromClass` "/Game/Object/BP_Box.BP_Box_C" (`KismetMathLibrary.Conv_VectorToTransform` (`SceneComponent.K2_GetComponentLocation` (`self.Box`))) "Undefined" "MultiplyWithRoot" null (`KismetArrayLibrary.Array_Random` (`|MakeArray` 1.0 2.0 3.0 5.0 :!type "Float (single-precision)")) (`KismetMathLibrary.Conv_IntToDouble` (`KismetMathLibrary.RandomIntegerInRange` 1 10)) null))
  (bind _output_get (set `self.SpawnedBox` _returnvalue))
  (set `self.taken` false)
  (`PrimitiveComponent.SetSimulatePhysics` (`/Game/Object/BP_Box.Cube` _output_get) false))

(event `self.Box.OnComponentEndOverlap`
  (params (OverlappedComponent :type "PrimitiveComponent Object Reference") (OtherActor :type "Actor Object Reference") (OtherComp :type "PrimitiveComponent Object Reference") (OtherBodyIndex :type Integer))
  (if (== OtherActor (`self.SpawnedBox`))
    (set `self.SpawnedBox` null)
    (set `self.taken` true)))

(fn `UserConstructionScript`)