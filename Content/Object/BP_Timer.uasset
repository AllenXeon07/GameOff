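; BP_Timer is a countdown clock actor that displays the match's remaining time from GM_MainGame.
; It caches the game mode at BeginPlay and polls TimeRemain on Tick, refreshing only when the whole second changes.
; SetTime builds a zero-padded minutes:seconds string for the Time text, and a 2D countdown sound plays on each update under ten seconds.
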(event `self.ReceiveBeginPlay`
  (bind _asgm_main_game (cast `/Game/Player/GM_MainGame` (`GameplayStatics.GetGameMode`)))
  (set `self.GameMode` _asgm_main_game))

(event `self.ReceiveTick`
  (params (DeltaSeconds :type "Float (single-precision)"))
  (bind _timeremain (`/Game/Player/GM_MainGame.TimeRemain` (`self.GameMode`)))
  (bind _returnvalue (`KismetMathLibrary.FFloor` _timeremain))
  (if (!= (`self.LastTime`) _returnvalue)
    (`self.SetTime` _timeremain)
    (bind _output_get (set `self.LastTime` _returnvalue))
    (if (< _output_get 10)
      (`GameplayStatics.PlaySound2D` "/Game/Sound/countdown2_revision_.countdown2_revision_" 1.0 1.0 0.0 null null))))

(fn `SetTime`
  (params (Time :type "Float (double-precision)"))
  (locals (TimeString :type String))
  (bind _returnvalue (`KismetMathLibrary.FFloor64` Time))
  (bind _returnvalue_2 (`KismetStringLibrary.Conv_Int64ToString` (mod _returnvalue 60)))
  (bind _returnvalue_3 (`KismetStringLibrary.Conv_Int64ToString` (/ _returnvalue 60.0)))
  (if (< (`KismetStringLibrary.Len` _returnvalue_3) 2)
    (set `local.TimeString` (`KismetStringLibrary.Concat_StrStr` (`local.TimeString`) "0" _returnvalue_3 ":"))
    (else
      (set `local.TimeString` (`KismetStringLibrary.Concat_StrStr` (`local.TimeString`) _returnvalue_3 ":"))))
  (if (< (`KismetStringLibrary.Len` _returnvalue_2) 2)
    (set `local.TimeString` (`KismetStringLibrary.Concat_StrStr` (`local.TimeString`) "0" _returnvalue_2))
    (else
      (set `local.TimeString` (`KismetStringLibrary.Concat_StrStr` (`local.TimeString`) _returnvalue_2))))
  (`TextRenderComponent.K2_SetText` (`self.Time`) (`KismetTextLibrary.Conv_StringToText` (`local.TimeString`))))

(fn `UserConstructionScript`)