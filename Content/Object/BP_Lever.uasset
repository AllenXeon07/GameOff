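; BP_Lever is an interactable lever that sends its linked Crate and displays that crate's current capacity, maximum capacity and score.
; Box overlap binds Interact to the player's interact event dispatcher and unbinds it when the player leaves.
; Interact plays a timeline that swings the handle and calls Send on the Crate past halfway, if not already sent.
; Tick refreshes the three text displays every frame.
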(event `self.ReceiveTick`
  (params (DeltaSeconds :type "Float (single-precision)"))
  (bind _crate (`self.Crate`))
  (`self.SetText` (`KismetMathLibrary.FTrunc` (`/Game/Object/BP_Crate.CurrentCapacity` _crate)) (`KismetMathLibrary.FTrunc` (`/Game/Object/BP_Crate.MaxCapacity` _crate)) (`KismetMathLibrary.FTrunc` (`/Game/Object/BP_Crate.Point` _crate))))

(event `self.Box.OnComponentBeginOverlap`
  (params (OverlappedComponent :type "PrimitiveComponent Object Reference") (OtherActor :type "Actor Object Reference") (OtherComp :type "PrimitiveComponent Object Reference") (OtherBodyIndex :type Integer) (bFromSweep :type Boolean) (SweepResult :type "HitResult Structure (by ref)"))
  (bind _asbp_player (cast `/Game/Player/BP_Player` OtherActor))
  (set `self.Player` _asbp_player)
  (add `/Game/Player/BP_Player.ED_Interact` (`self.Player`) (delegate `Interact`)))

(event `self.Box.OnComponentEndOverlap`
  (params (OverlappedComponent :type "PrimitiveComponent Object Reference") (OtherActor :type "Actor Object Reference") (OtherComp :type "PrimitiveComponent Object Reference") (OtherBodyIndex :type Integer))
  (cast `/Game/Player/BP_Player` OtherActor)
  (`/Engine/EditorBlueprintResources/StandardMacros.IsValid` (`self.Player`)
    (:`Is Valid`
      (remove `/Game/Player/BP_Player.ED_Interact` (`self.Player`) (delegate `Interact`))
      (set `self.Player` null))))

(event `Interact`
  (bind _crate (`self.Crate`))
  (if (not (and (`self.Run?`) (not (`/Game/Object/BP_Crate.Send?` (`self.Crate`)))))
    (set `self.Run?` true)
    (bind (_direction _alpha) (`Timeline|TimelineInteractive` :!via `PlayFromStart`)
      (:`Update`
        (`SceneComponent.K2_SetRelativeRotation` (`self.switcher_handle`) (`KismetMathLibrary.MakeRotator` (`KismetMathLibrary.Lerp` -45.0 45.0 _alpha)) false false)
        (if (and (> _alpha 0.5) (not (`/Game/Object/BP_Crate.Send?` _crate)))
          (`/Game/Object/BP_Crate.Send` _crate)))
      (:`Finished`
        (set `self.Run?` false)))))

(fn `SetText`
  (params (Current :type Integer) (Max :type Integer) (Point :type Integer))
  (`TextRenderComponent.K2_SetText` (`self.CurrentCap`) (`KismetTextLibrary.Conv_IntToText` Current))
  (`TextRenderComponent.K2_SetText` (`self.MaxCap`) (`KismetTextLibrary.Conv_IntToText` Max))
  (`TextRenderComponent.K2_SetText` (`self.Score`) (`KismetTextLibrary.Conv_IntToText` Point)))

(fn `UserConstructionScript`)