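; BP_RandomBox is a box actor marked with a white "?" text, configured entirely in its construction script.
; The script creates a dynamic instance of MI_RandomColor, sets it fully opaque and applies it to one material slot of the cube.
; It also overrides the cube's mass with a scaled Mass variable.
; The event graph holds only disabled stub events, so the Blueprint adds no runtime logic.
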(fn `UserConstructionScript`
  (bind _textrender (`self.TextRender`))
  (bind _returnvalue (`KismetMaterialLibrary.CreateDynamicMaterialInstance` "/Game/Object/MI_RandomColor.MI_RandomColor"))
  (set `self.Material` _returnvalue)
  (`MaterialInstanceDynamic.SetScalarParameterValue` _returnvalue "Opacity" 1.0)
  (`PrimitiveComponent.SetMaterial` (`self.Cube`) 2 (`self.Material`))
  (`PrimitiveComponent.SetMassOverrideInKg` (`self.Cube`) "None" (* (`self.Mass`) 500.0) true)
  (`TextRenderComponent.K2_SetText` _textrender (`KismetTextLibrary.Conv_StringToText` "?"))
  (`TextRenderComponent.SetTextRenderColor` _textrender (make `Color` 255 255 255 255)))