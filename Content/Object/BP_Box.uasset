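; BP_Box is a physics box that players carry and throw, showing a point value and fading out until destroyed if left uncarried too long.
; Construction sets color and physical weight from Mass.
; Overlapping binds Interact to the player's dispatcher, which attaches the box to the Carry socket, resets its lifetime and binds Release.
; Release detaches it, launches it along the player-to-socket direction at a speed inversely proportional to Mass, then clears bindings.
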(event `self.Box.OnComponentEndOverlap`
  (params (OverlappedComponent :type "PrimitiveComponent Object Reference") (OtherActor :type "Actor Object Reference") (OtherComp :type "PrimitiveComponent Object Reference") (OtherBodyIndex :type Integer))
  (bind _asbp_player (cast `/Game/Player/BP_Player` OtherActor))
  (clear `/Game/Player/BP_Player.ED_Interact` _asbp_player))

(event `self.Box.OnComponentBeginOverlap`
  (params (OverlappedComponent :type "PrimitiveComponent Object Reference") (OtherActor :type "Actor Object Reference") (OtherComp :type "PrimitiveComponent Object Reference") (OtherBodyIndex :type Integer) (bFromSweep :type Boolean) (SweepResult :type "HitResult Structure (by ref)"))
  (bind _asbp_player (cast `/Game/Player/BP_Player` OtherActor))
  (bind _output_get (set `self.Player` _asbp_player))
  (add `/Game/Player/BP_Player.ED_Interact` _output_get (delegate `Interact`)))

(event `self.ReceiveTick`
  (params (DeltaSeconds :type "Float (single-precision)"))
  (bind _maxlifetime (`self.maxLifeTime`))
  (if (not (`self.take`))
    (bind _output_get (set `self.currentLifeTime` (+ (`self.currentLifeTime`) DeltaSeconds)))
    (`MaterialInstanceDynamic.SetScalarParameterValue` (`self.Material`) "Opacity" (- 1.0 (`KismetMathLibrary.MultiplyMultiply_FloatFloat` (/ _output_get _maxlifetime) 5.0)))
    (if (>= _output_get _maxlifetime)
      (`self.K2_DestroyActor`))
    (else
      (`MaterialInstanceDynamic.SetScalarParameterValue` (`self.Material`) "Opacity" 1.0))))

(event `self.ReceiveBeginPlay`)

(event `Interact`
  (bind _player (`self.Player`))
  (`/Game/Player/BP_Player.SetEmote` _player "Heavy")
  (`Character.PlayAnimMontage` _player "/Game/Player/Anim/AM_Carry.AM_Carry" 1.0 "None")
  (set `self.take` true)
  (set `self.currentLifeTime` 0.0)
  (if (not (`/Game/Player/BP_Player.Carry` (`self.Player`)))
    (add `/Game/Player/BP_Player.ED_Release` (`self.Player`) (delegate `Release`))
    (set `/Game/Player/BP_Player.Carry` true (`self.Player`))
    (`PrimitiveComponent.SetSimulatePhysics` (`self.Cube`) false)
    (`self.K2_AttachToComponent` (`Character.Mesh` (`self.Player`)) "Carry" "SnapToTarget" "KeepWorld" "KeepWorld")
    (`KismetSystemLibrary.MoveComponentTo` (`self.Cube`) (0.0 0.0 0.0) (struct) true true 0.0 true)
    (`self.SetActorEnableCollision` false)))

(event `Release`
  (bind _player (`self.Player`))
  (bind _player_2 (`self.Player`))
  (`/Game/Player/BP_Player.SetEmote` (`self.Player`) "Suprised")
  (`Character.StopAnimMontage` (`self.Player`) "/Game/Player/Anim/AM_Carry.AM_Carry")
  (`self.K2_DetachFromActor` "KeepRelative" "KeepRelative" "KeepWorld")
  (set `self.take` false)
  (set `/Game/Player/BP_Player.Carry` false (`self.Player`))
  (`PrimitiveComponent.SetSimulatePhysics` (`self.Cube`) true)
  (`self.SetActorEnableCollision` true)
  (`PrimitiveComponent.SetPhysicsLinearVelocity` (`self.Cube`) (* (`KismetMathLibrary.GetDirectionUnitVector` (`self.K2_GetActorLocation` _player) (`SceneComponent.GetSocketLocation` (`Character.Mesh` _player) "Carry")) (`self.Speed`) (/ 1.0 (* (`self.Mass`) 30.0))) false "None")
  (`KismetSystemLibrary.Delay` 0.1)
  (clear `/Game/Player/BP_Player.ED_Interact` _player_2)
  (clear `/Game/Player/BP_Player.ED_Release` _player_2)
  (set `self.Temp_player` (`self.Player`))
  (set `self.Player` null)
  (`KismetSystemLibrary.Delay` 2.0)
  (`/Game/Player/BP_Player.SetEmote` (`self.Temp_player`) "Neutral")
  (set `self.Temp_player` null))

(fn `UserConstructionScript`
  (bind _textrender (`self.TextRender`))
  (bind _value (`BlueprintMapLibrary.Map_Find` (`self.ListColor`) (`self.Mass`)))
  (bind _returnvalue (`KismetMaterialLibrary.CreateDynamicMaterialInstance` "/Game/Object/MI_Color.MI_Color"))
  (set `self.Material` _returnvalue)
  (`MaterialInstanceDynamic.SetVectorParameterValue` _returnvalue "Base Color" _value)
  (`MaterialInstanceDynamic.SetScalarParameterValue` _returnvalue "Opacity" 1.0)
  (`PrimitiveComponent.SetMaterial` (`self.Cube`) 2 (`self.Material`))
  (`PrimitiveComponent.SetMassOverrideInKg` (`self.Cube`) "None" (* (`self.Mass`) 10.0) true)
  (`TextRenderComponent.K2_SetText` _textrender (`KismetTextLibrary.Conv_DoubleToText` (`self.Point`) "HalfToEven"))
  (`TextRenderComponent.SetTextRenderColor` _textrender (`KismetMathLibrary.Conv_LinearColorToColor` _value)))